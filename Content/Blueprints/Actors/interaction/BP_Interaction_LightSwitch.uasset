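; Interactable light switch actor that toggles a linked light on and off.
; On Interact, it flips the visibility of the referenced Light's LightComponent if it is valid.
; BeginPlay caches the player as an L1_Character reference, which the toggle logic does not use.
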(event `self.ReceiveBeginPlay`
  (`self.GetPlayerRef`))

(event `/Game/Blueprints/Interfaces/BPI_Interaction.Interact`
  (bind _light (`self.Light`))
  (bind _lightcomponent (`Light.LightComponent` _light))
  (bind _lightcomponent_2 (`Light.LightComponent` _light))
  (`/Engine/EditorBlueprintResources/StandardMacros.IsValid` _lightcomponent_2
    (:`Is Valid`
      (if (`SceneComponent.IsVisible` _lightcomponent_2)
        (`SceneComponent.SetVisibility` _lightcomponent false false)
        (else
          (`SceneComponent.SetVisibility` _lightcomponent true false))))))

(fn `GetPlayerRef`
  (bind _asl1_character (cast `/Game/GameBlueprints/Level1/L1_Character` (`GameplayStatics.GetPlayerCharacter` 0)))
  (set `self.PlayerRef` _asl1_character))

(fn `UserConstructionScript`)
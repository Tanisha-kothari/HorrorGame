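; Inventory component that stores item class and amount per slot, sized from the player controller's slot count.
; AddItem fills partial stacks, then empty slots, recursing on overflow and returning a remainder, though the non-stackable branch discards the recursive remainder.
; UseItem calls UseItem on an existing or newly spawned item actor, then removes one; DropItem empties the slot without spawning anything.
; Slot changes refresh the matching grid widget through the player controller.
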(event `self.ReceiveBeginPlay`
  (bind _ashg_player_controller (cast `/Game/GameBlueprints/HG_PlayerController` (`GameplayStatics.GetPlayerController` 0) :!pure true))
  (`KismetArrayLibrary.Array_Resize` (`self.InventorySlots`) (`/Game/GameBlueprints/HG_PlayerController.inventoryslots` _ashg_player_controller))
  (set `self.Inventory` (`/Game/GameBlueprints/HG_PlayerController.Inventory` _ashg_player_controller))
  (`KismetSystemLibrary.PrintString` "1 from BPC inventory event graph"))

(fn `AddItem`
  (params (Item :type "/Game/Blueprints/Actors/Inventory/BP_InventoryItemMaster Class Reference") (Amount :type Integer))
  (returns (Success :type Boolean) (Remainder :type Integer))
  (locals (LocalItem :type "/Game/Blueprints/Actors/Inventory/BP_InventoryItemMaster Class Reference") (LocalAmount :type Integer) (LocalMaxStackAmt :type Integer) (LocalIndex :type Integer :default 0))
  (bind (_success _index) (`self.CheckForEmptySlot`))
  (bind (_success_2 _index_2) (`self.CheckForEmptySlot`))
  (bind _returnvalue (- (`local.LocalAmount`) 1))
  (bind (_item_name _icon _maxstackamount) (break `/Game/Blueprints/Structs/S_ItemData` (defaults `Object` (`local.LocalItem`))))
  (`KismetSystemLibrary.PrintString` "2 from bpc inevntory add item function")
  (set `local.LocalItem` Item)
  (set `local.LocalAmount` Amount)
  (set `local.LocalMaxStackAmt` _maxstackamount)
  (if (> _maxstackamount 1)
    (bind (_success_ _index_3) (`self.CheckForSlotWithSpace` (`local.LocalItem`)))
    (if _success_
      (bind _output_get (set `local.LocalIndex` _index_3))
      (bind _returnvalue_2 (+ (`.Amount` (`self.GetItemDataAtIndex` _output_get)) (`local.LocalAmount`)))
      (if (> _returnvalue_2 (`local.LocalMaxStackAmt`))
        (set `local.LocalAmount` (- _returnvalue_2 (`local.LocalMaxStackAmt`)))
        (`KismetArrayLibrary.Array_Set` (`self.InventorySlots`) (`local.LocalIndex`) (make `/Game/Blueprints/Structs/S_InventoryItem` (`local.LocalMaxStackAmt`) (`local.LocalItem`)))
        (`self.UpdateInventorySlot` (`local.LocalIndex`))
        (bind (_success_3 _remainder) (`self.AddItem` (`local.LocalItem`) (`local.LocalAmount`)))
        (return true _remainder)
        (else
          (`KismetArrayLibrary.Array_Set` (`self.InventorySlots`) (`local.LocalIndex`) (make `/Game/Blueprints/Structs/S_InventoryItem` _returnvalue_2 (`local.LocalItem`)))
          (`self.UpdateInventorySlot` (`local.LocalIndex`))
          (return true 0)))
      (elif _success
        (set `local.LocalIndex` _index)
        (if (> (`local.LocalAmount`) (`local.LocalMaxStackAmt`))
          (`KismetArrayLibrary.Array_Set` (`self.InventorySlots`) (`local.LocalIndex`) (make `/Game/Blueprints/Structs/S_InventoryItem` (`local.LocalMaxStackAmt`) (`local.LocalItem`)))
          (`self.UpdateInventorySlot` (`local.LocalIndex`))
          (bind (_success_4 _remainder_2) (`self.AddItem` (`local.LocalItem`) (- (`local.LocalAmount`) (`local.LocalMaxStackAmt`))))
          (return true _remainder_2)
          (else
            (`KismetArrayLibrary.Array_Set` (`self.InventorySlots`) (`local.LocalIndex`) (make `/Game/Blueprints/Structs/S_InventoryItem` (`local.LocalAmount`) (`local.LocalItem`)))
            (`self.UpdateInventorySlot` (`local.LocalIndex`))
            (return true 0)))
        (else
          (return false (`local.LocalAmount`)))))
    (elif _success_2
      (set `local.LocalIndex` _index_2)
      (`KismetArrayLibrary.Array_Set` (`self.InventorySlots`) (`local.LocalIndex`) (make `/Game/Blueprints/Structs/S_InventoryItem` 1 (`local.LocalItem`)) true)
      (`self.UpdateInventorySlot` (`local.LocalIndex`))
      (if (> _returnvalue 0)
        (`self.AddItem` (`local.LocalItem`) _returnvalue)
        (return true 0)
        (else
          (return true 0)))
      (else
        (`KismetSystemLibrary.PrintString` "No free slots")
        (return false (`local.LocalAmount`))))))

(fn `CheckForEmptySlot`
  (returns (Success :type Boolean) (Index :type Integer))
  (locals (LocalSuccess :type Boolean) (localindex :type Integer))
  (for (_array_element _array_index) (`self.InventorySlots`)
    (if (`KismetSystemLibrary.IsValidClass` (`.Item_9_DF48FDEF4DB6060A04562298AB730150` (break `/Game/Blueprints/Structs/S_InventoryItem` _array_element)))
      (set `local.LocalSuccess` false)
      (else
        (set `local.LocalSuccess` true)
        (set `local.localindex` _array_index)
        (break))))
  (return (`local.LocalSuccess`) (`local.localindex`)))

(fn `CheckForSlotWithSpace`
  (params (item :type "/Game/Blueprints/Actors/Inventory/BP_InventoryItemMaster Class Reference"))
  (returns (`success?` :type Boolean) (index :type Integer))
  (locals (LocalSuccess :type Boolean) (LocalIndex :type Integer))
  (for (_array_element _array_index) (`self.InventorySlots`)
    (bind (_amount _item) (break `/Game/Blueprints/Structs/S_InventoryItem` _array_element))
    (if (and (== _item item) (< _amount (`.MaxStackAmount_8_4A62C16044A763BD85E12588C6271722` (break `/Game/Blueprints/Structs/S_ItemData` (defaults `Object` item)))))
      (set `local.LocalSuccess` true)
      (set `local.LocalIndex` _array_index)
      (break)
      (else
        (set `local.LocalSuccess` false))))
  (return (`local.LocalSuccess`) (`local.LocalIndex`)))

(fn `DropItem`
  (params (`Local Index` :type Integer))
  (locals (localIndex :type Integer) (localamout :type Integer :default 0))
  (bind _output_get (set `local.localIndex` `Local Index`))
  (set `local.localamout` (`.Amount` (`self.GetItemDataAtIndex` _output_get)))
  (if (> (`local.localamout`) 0)
    (for _ (range (`local.localamout`))
      (`self.RemoveItem` (`local.localIndex`)))
    (`/Game/Blueprints/UI/Inventory/W_InventoryMenu.CloseDropDownMenu` (`self.Inventory`))))

(fn `GetItemDataAtIndex`
  (params (Index :type Integer))
  (returns (Item :type "/Game/Blueprints/Actors/Inventory/BP_InventoryItemMaster Class Reference") (Amount :type Integer))
  (bind (_amount _item) (break `/Game/Blueprints/Structs/S_InventoryItem` (`|GetArrayItem` (`self.InventorySlots`) Index)))
  (return _item _amount))

(fn `RemoveItem`
  (params (Index :type Integer))
  (bind (_item _amount) (`self.GetItemDataAtIndex` Index))
  (set `self.Index` Index)
  (if (> _amount 1)
    (`KismetArrayLibrary.Array_Set` (`self.InventorySlots`) (`self.Index`) (make `/Game/Blueprints/Structs/S_InventoryItem` (- _amount 1) _item) true)
    (else
      (`KismetArrayLibrary.Array_Set` (`self.InventorySlots`) (`self.Index`) (make `/Game/Blueprints/Structs/S_InventoryItem` 0))))
  (`self.UpdateInventorySlot` (`self.Index`)))

(fn `UpdateInventorySlot`
  (params (Index :type Integer))
  (`/Game/Blueprints/UI/Inventory/W_InventorySlot.UpdateSlot` (`|GetArrayItem` (`/Game/Blueprints/UI/Inventory/W_inventoryGrid.SlotsArray` (`/Game/Blueprints/UI/Inventory/W_InventoryMenu.W_inventoryGrid` (`/Game/GameBlueprints/HG_PlayerController.Inventory` (cast `/Game/GameBlueprints/HG_PlayerController` (`GameplayStatics.GetPlayerController` 0) :!pure true)))) Index)))

(fn `UseItem`
  (params (Index :type Integer))
  (locals (LocalIndex :type Integer) (NewLocalVar :type Boolean))
  (bind _output_get (set `local.LocalIndex` Index))
  (bind (_item _amount) (`self.GetItemDataAtIndex` _output_get))
  (if (> _amount 0)
    (bind _returnvalue (`GameplayStatics.GetActorOfClass` _item))
    (`/Engine/EditorBlueprintResources/StandardMacros.IsValid` _returnvalue
      (:`Is Valid`
        (`/Game/Blueprints/Actors/Inventory/BP_InventoryItemMaster.UseItem` _returnvalue))
      (:`Is Not Valid`
        (bind _returnvalue_2 (`|SpawnActorFromClass` _item (`KismetMathLibrary.MakeTransform` (0.0 0.0 0.0)) "Undefined" "MultiplyWithRoot" null null))
        (`/Game/Blueprints/Actors/Inventory/BP_InventoryItemMaster.UseItem` _returnvalue_2)))
    (`self.RemoveItem` _output_get)
    (`/Game/Blueprints/UI/Inventory/W_InventoryMenu.CloseDropDownMenu` (`self.Inventory`))))
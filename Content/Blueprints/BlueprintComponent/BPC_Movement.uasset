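; Movement component for the player character that handles stamina-limited sprinting and crouching by changing max walk speed.
; Looping timers drain stamina while sprinting and refill it after a retriggerable delay once sprint stops, printing the value on each change.
; Crouching cancels the sprint timer and calls L1_Character to run its crouch timeline or lengthen the capsule on standing.
; Initialize stores the character reference and applies walk speed.
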(event `StartSprint`
  (if (`self.IsCrouching`)
    (`self.StopCrouch`))
  (if (and (> (`self.CurrentStamina`) (`self.MinStamina`)) (> (`KismetMathLibrary.VSize` (`Actor.GetVelocity` (`self.PlayerRef`))) 0.0))
    (`KismetSystemLibrary.K2_ClearTimer` null "RegenrateStamina")
    (`self.SetPlayerMaxWalkSpeed` (`self.SprintSpeed`))
    (`KismetSystemLibrary.K2_SetTimer` null "SprintTime" 0.1 true)))

(event `SprintTime`
  (if (> (`KismetMathLibrary.VSize` (`Actor.GetVelocity` (`self.PlayerRef`))) 0.0)
    (bind _output_get (set `self.CurrentStamina` (`KismetMathLibrary.FClamp` (- (`self.CurrentStamina`) 1.0) (`self.MinStamina`) (`self.MaxStamina`))))
    (`KismetSystemLibrary.PrintString` (`KismetStringLibrary.Conv_DoubleToString` _output_get))
    (if (<= (`self.CurrentStamina`) (`self.MinStamina`))
      (`self.StopSprint`))
    (else
      (`self.StopSprint`))))

(event `StopSprint`
  (if (not (`self.IsCrouching`))
    (`KismetSystemLibrary.K2_ClearTimer` null "SprintTime")
    (`self.SetPlayerMaxWalkSpeed` (`self.WalkSpeed`))
    (`KismetSystemLibrary.RetriggerableDelay` 5.0)
    (if (not (`KismetSystemLibrary.K2_IsTimerActive` null "SprintTimer"))
      (`KismetSystemLibrary.K2_SetTimer` null "RegenrateStamina" 0.03 true))))

(event `RegenrateStamina`
  (bind _output_get (set `self.CurrentStamina` (`KismetMathLibrary.FClamp` (+ (`self.CurrentStamina`) 1.0) (`self.MinStamina`) (`self.MaxStamina`))))
  (`KismetSystemLibrary.PrintString` (`KismetStringLibrary.Conv_DoubleToString` _output_get))
  (if (== (`self.CurrentStamina`) (`self.MaxStamina`))
    (`KismetSystemLibrary.K2_ClearTimer` null "RegenrateStamina")))

(event `StartCrouch`
  (`KismetSystemLibrary.K2_ClearTimer` null "SprintTime")
  (`self.SetPlayerMaxWalkSpeed` (`self.Crouch Speed`))
  (`/Game/GameBlueprints/Level1/L1_Character.CrouchTimeline` (cast `/Game/GameBlueprints/Level1/L1_Character` (`self.PlayerRef`) :!pure true))
  (set `self.IsCrouching` true))

(event `StopCrouch`
  (`self.SetPlayerMaxWalkSpeed` (`self.WalkSpeed`))
  (`/Game/GameBlueprints/Level1/L1_Character.LengthenPlayerCapsule` (cast `/Game/GameBlueprints/Level1/L1_Character` (`self.PlayerRef`) :!pure true))
  (set `self.IsCrouching` false))

(fn `Initialize`
  (params (character :type "Character Object Reference"))
  (set `self.PlayerRef` character)
  (set `CharacterMovementComponent.MaxWalkSpeed` (`self.WalkSpeed`) (`Character.CharacterMovement` (`self.PlayerRef`))))

(fn `SetPlayerMaxWalkSpeed`
  (params (MaxWalkSpeed :type "Float (single-precision)"))
  (set `CharacterMovementComponent.MaxWalkSpeed` MaxWalkSpeed (`Character.CharacterMovement` (`self.PlayerRef`))))